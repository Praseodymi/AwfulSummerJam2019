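; End door that swings open when the player overlaps its trigger box while holding the key.
; The box overlap checks the HasKey flag on the ASJ19 game instance, then plays the DoorOpen timeline.
; The timeline's Angle track rotates the two door leaves 90 degrees in opposite directions.
; A DoOnce on the timeline update plays the creaky door sound a single time.
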(event OnComponentBeginOverlap(Box)
  (params (OverlappedComponent :type Primitive%20Component%20Object%20Reference) (OtherActor :type Actor%20Object%20Reference) (OtherComp :type Primitive%20Component%20Object%20Reference) (OtherBodyIndex :type Integer) (bFromSweep :type Boolean) (SweepResult :type Hit%20Result%20Structure%20%28by%20ref%29))
  (if (== OtherActor (Game|GetPlayerCharacter 0))
    (bind _asasj19_game_instance (Utilities|Casting|CastToASJ19_GameInstance (Game|GetGameInstance)))
    (if (Variables|/Game/Levels/ASJ19_GameInstance.ASJ19_GameInstance_C|GetHasKey _asasj19_game_instance)
      (bind _angle (Timeline|DoorOpen Play)
        (:Update
          (Transformation|SetRelativeRotation (Variables|Default|GetDoorR) (Math|Rotator|Lerp(Rotator) "0, 0, 0" "0.000000,90.000000, 0" _angle true) false false)
          (Transformation|SetRelativeRotation (Variables|Default|GetDoorL) (Math|Rotator|Lerp(Rotator) "0, 0, 0" "0.000000,-90.000000, 0" _angle true) false false)
          (Utilities|FlowControl|DoOnce false
            (:Completed
              (Audio|PlaySound2D "/Game/Audio/SFX/452708__parkersenk__creaky-door.452708__parkersenk__creaky-door" 1.0 1.0 0.0 0 0))))))))

(fn ConstructionScript)