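; MagicTrap is a trap actor that fires a magic shot effect toward the player on demand.
; Fire spawns a BP_ky_shotSpawn at the ParticleSystem1 component, rotated once at spawn to face the first player character, and stores it in ShotRef.
; StopFiring destroys that stored spawn if it is still valid; neither event is triggered within this graph.
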(event Custom|StopFiring
  (bind _shotref (Variables|Default|GetShotRef))
  (Utilities|IsValid _shotref
    (:Is%20Valid
      (Actor|DestroyActor _shotref))))

(event Custom|Fire
  (bind _returnvalue (Game|SpawnActorfromClass "/Game/FXVarietyPack/Blueprints/BP_ky_shotSpawn.BP_ky_shotSpawn_C" (Math|Transform|MakeTransform (Transformation|GetWorldLocation (Variables|Default|GetParticleSystem1)) (Math|Rotator|FindLookatRotation (Transformation|GetWorldLocation (Variables|Default|GetParticleSystem1)) (Transformation|GetWorldLocation (Variables|/Script/Engine.Actor|GetRootComponent (Game|GetPlayerCharacter 0))))) "Undefined" 0 0))
  (Variables|Default|SetShotRef _returnvalue))

(fn ConstructionScript)