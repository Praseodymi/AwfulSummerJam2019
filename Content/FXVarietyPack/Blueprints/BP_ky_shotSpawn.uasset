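; BP_ky_shotSpawn is an effect spawner from the FX Variety Pack that fires a Shot actor from its own transform.
; BeginPlay spawns the shot, then either repeats on a fixed delay when IsLoop is set or destroys itself after the single spawn.
; Tick continuously rotates the spawner to face the first player character, so later shots launch toward the player.
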(event EventBeginPlay
  ;[1 1 1] spawn shot
  (Game|SpawnActorfromClass (Variables|Default|Getshot) (Transformation|GetActorTransform) "Undefined" 0 0 :!label _label)
  ;[1 1 1] repeat control
  (if (Variables|Default|GetisLoop)
    (Utilities|FlowControl|Delay 5.0)
    (goto _label)
    (else
      ;[1 1 1] destroy
      (Actor|DestroyActor))))

(event EventTick
  (params (DeltaSeconds :type Float%20%28single-precision%29))
  ;[1 1 1] rotation control
  (Transformation|SetActorRotation (Math|Rotator|FindLookatRotation (Transformation|GetActorLocation) (Transformation|GetWorldLocation (Variables|/Script/Engine.Actor|GetRootComponent (Game|GetPlayerCharacter 0))))))

(fn ConstructionScript)